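; Tank Blueprint that, as shown, handles only an orbit camera driven by player input axes.
; Aim axes add local yaw to an azimuth gimbal and local pitch to an elevation spring arm, keeping the two rotations on separate components.
; A camera distance axis zooms by changing the arm length, with step, starting length and clamp limits all scaled from one delta set at BeginPlay.
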(event `self.ReceiveBeginPlay`
  ;[1 1 1] Initialization of ArmLength
  (bind _output_get (set `self.ArmLengthDelta` 500.0))
  (set `SpringArmComponent.TargetArmLength` (* _output_get 0.5) (`self.ElevationGimbal`)))

(event `InputAxis|AimElevation`
  (params (AxisValue :type "Float (single-precision)"))
  ;[1 1 1] Camera Input Binding
  (`SceneComponent.K2_AddLocalRotation` (`self.ElevationGimbal`) (`KismetMathLibrary.MakeRotator` 0.0 AxisValue) false false))

(event `InputAxis|AimAzimuth`
  (params (AxisValue :type "Float (single-precision)"))
  ;[1 1 1] Camera Input Binding
  (`SceneComponent.K2_AddLocalRotation` (`self.AzimuthGimbal`) (`KismetMathLibrary.MakeRotator` 0.0 0.0 AxisValue) false false))

(event `InputAxis|CameraDistance`
  (params (AxisValue :type "Float (single-precision)"))
  (bind _armlengthdelta (`self.ArmLengthDelta`))
  (bind _elevationgimbal (`self.ElevationGimbal`))
  ;[1 1 1] Camera Input Binding
  (set `SpringArmComponent.TargetArmLength` (`KismetMathLibrary.FClamp` (- (`SpringArmComponent.TargetArmLength` _elevationgimbal) (* AxisValue (`self.ArmLengthDelta`))) (* _armlengthdelta -0.5) (* _armlengthdelta 3.5)) _elevationgimbal))

(fn `UserConstructionScript`)